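; BP_GameMode is a game mode that runs the game timer and displays the HUD.
; On BeginPlay it starts a looping one-second timer that calls gameTimer to add to the Timer value, then creates W_HUD and adds it to the viewport.
; Tick passes through a one-second Delay, then formats the Timer's minutes and seconds into the TimerToText variable.
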(event `self.ReceiveTick`
  (params (DeltaSeconds :type "Float (single-precision)"))
  (bind (_days _hours _minutes _seconds) (`KismetMathLibrary.BreakTimespan` (`self.timer`)))
  ;[0.1333 0.1333 0.1333] Game Timer
  (`KismetSystemLibrary.Delay` 1.0)
  (set `self.timerToText` (`|FormatText` "{m}:{s}" (`KismetTextLibrary.Conv_IntToText` _minutes false true 2 2) (`KismetTextLibrary.Conv_IntToText` _seconds false true 2 2))))

(event `self.ReceiveBeginPlay`
  (`|ExecutionSequence`
    (:`then_0`
      ;[0.1333 0.1333 0.1333] Game Timer
      (`KismetSystemLibrary.K2_SetTimer` null "gameTimer" 1.0 true))
    (:`then_1`
      ;[0 0.9162 1] Display HUD
      (bind _returnvalue (`|CreateWidget` "/Game/Blueprints_FromModProject/Widgets/W_HUD.W_HUD_C"))
      (bind _output_get (set `self.W_HUD_ref` _returnvalue))
      (`UserWidget.AddToViewport` _output_get 0))))

(fn `gameTimer`
  (set `self.timer` (+ (`self.timer`) (`self.seconds`))))

(fn `UserConstructionScript`)