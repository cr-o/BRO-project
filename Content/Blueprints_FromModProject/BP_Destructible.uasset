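; BP_Destructible is an actor that breaks after the third-person character touches it enough times.
; Each overlap of its Sphere by BP_ThirdPersonCharacter decrements HitsRemaining and prints the new count on screen.
; At zero it plays a sound at its location, destroys itself and calls ObjectiveChecker on BP_GameMode.
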(event `self.Sphere.OnComponentBeginOverlap`
  (params (OverlappedComponent :type "PrimitiveComponent Object Reference") (OtherActor :type "Actor Object Reference") (OtherComp :type "PrimitiveComponent Object Reference") (OtherBodyIndex :type Integer) (bFromSweep :type Boolean) (SweepResult :type "HitResult Structure (by ref)"))
  ;[1 1 1] Destroy items after a certain amount of hits, then update counter on HUD and call objective checker
  (cast `/Game/ThirdPerson/Blueprints/BP_ThirdPersonCharacter` OtherActor)
  (bind _result (`/Engine/EditorBlueprintResources/StandardMacros.DecrementInt` (`self.hitsRemaining`))
    (:`  `
      (bind _output_get (set `self.hitsRemaining` _result))
      (`KismetSystemLibrary.PrintString` (`KismetStringLibrary.Conv_IntToString` _output_get))
      (if (== (`self.hitsRemaining`) 0)
        (`GameplayStatics.PlaySoundAtLocation` "/Game/Imported/Sounds/placeblock.placeblock" (`self.K2_GetActorLocation`) (struct) 1.0 1.0 0.0 null null null null)
        (`self.K2_DestroyActor`)
        (bind _asbp_game_mode (cast `/Game/Blueprints_FromModProject/BP_GameMode` (`GameplayStatics.GetGameMode`)))
        (`/Game/Blueprints_FromModProject/BP_GameMode.objectiveChecker` _asbp_game_mode)))))

(fn `UserConstructionScript`)