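; BP_GameMode is the game mode that runs a countdown timer and shows it on the HUD.
; On BeginPlay it creates the W_HUD widget, adds it to the viewport and starts a looping one-second timer that calls gameTimer to decrement Timer.
; Tick formats the remaining minutes and seconds into TimerText and tells the HUD to update every frame.
; No handling for the countdown reaching zero is present.
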(event `self.ReceiveBeginPlay`
  (`|ExecutionSequence`
    (:`then_0`
      ;[1 1 1] Display HUD
      (bind _returnvalue (`|CreateWidget` "/Game/Blueprints/Widgets/W_HUD.W_HUD_C"))
      (bind _output_get (set `self.HUD_ref` _returnvalue))
      (`UserWidget.AddToViewport` _output_get 0))
    (:`then_1`
      ;[1 1 1] Game Timer
      (`KismetSystemLibrary.K2_SetTimer` null "gameTimer" 1.0 true))))

(event `self.ReceiveTick`
  (params (DeltaSeconds :type "Float (single-precision)"))
  (bind (_days _hours _minutes _seconds) (`KismetMathLibrary.BreakTimespan` (`self.timer`)))
  ;[1 1 1] Game Timer
  (set `self.timerText` (`|FormatText` "{m}:{s}" (`KismetTextLibrary.Conv_IntToText` _minutes false true 2) (`KismetTextLibrary.Conv_IntToText` _seconds false true 2)))
  (`/Game/Blueprints/Widgets/W_HUD.updateTimer` (`self.HUD_ref`)))

(fn `gameTimer`
  (set `self.timer` (- (`self.timer`) (`self.seconds`))))

(fn `UserConstructionScript`)