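; BP_NPC02 is a placed NPC that shows and cycles through dialogue when the player talks to it nearby.
; Beginning an overlap prints an interact prompt, and the Talk event calls DisplayDialogue, whose body is not in this file.
; When the player character leaves while the dialogue widget is valid, it removes the widget, sets WalkedAway, and destroys the NPC if no lines remain.
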(event `/Game/Blueprints/BPI_Dialogue.Talk`
  ;[1 1 1] NPC PLACED IN WORLD. When you "talk" using the interact input when you're near enough to it, display and cycle through dialogue.
  (`self.displayDialogue`))

(event `self.ReceiveActorEndOverlap`
  (params (OtherActor :type "Actor Object Reference"))
  ;[1 1 1] Remove dialogue UI if player walks away
  (`self.WDialogueRef`
    (:`then`
      (cast `/Game/Blueprints/BP_3PCHAR` OtherActor)
      (`Widget.RemoveFromParent` (`self.WDialogueRef`))
      (set `self.walkedAway` true)
      ;[1 1 1] If no dialogue left when you walk away, NPC just goes away
      (if (not (< (`self.talkIndex`) (`KismetArrayLibrary.Array_Length` (`self.dialogue`))))
        (`self.K2_DestroyActor`)))
    (:`else`)))

(event `self.ReceiveActorBeginOverlap`
  (params (OtherActor :type "Actor Object Reference"))
  ;[1 1 1] Prompt player to talk when close enough to NPC
  (`KismetSystemLibrary.PrintString` "Press E to talk"))

(fn `NewFunction_0_0`)

(fn `UserConstructionScript`
  (`parent.UserConstructionScript`))